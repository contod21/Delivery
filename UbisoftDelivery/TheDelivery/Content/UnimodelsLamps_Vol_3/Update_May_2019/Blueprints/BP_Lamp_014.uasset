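; BP_Lamp_014 is a lamp prop Blueprint with an adjustable point light and a matching emissive bulb.
; The construction script applies intensity, temperature and attenuation radius variables to the PointLight.
; It also creates a dynamic instance of an emissive material on the LightBulb001 mesh and feeds it the same intensity, so the bulb glow follows the light.
; The event graph holds only disabled stubs, with no runtime logic.
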(event EventBeginPlay)

(event Collision|EventActorBeginOverlap
  (params (OtherActor :type Actor%20Object%20Reference)))

(event EventTick
  (params (DeltaSeconds :type Float%20%28single-precision%29)))

(fn ConstructionScript
  (bind _pointlight (Variables|Default|GetPointLight))
  (Rendering|Components|Light|SetIntensity _pointlight (Variables|Default|GetLight_Intensity))
  (Class|LightComponent|SetTemperature _pointlight (Variables|Default|GetLight_Temp))
  (bind _returnvalue (Rendering|Material|CreateDynamicMaterialInstance (Variables|Default|GetLightBulb_001) 2 "/Game/UnimodelsLamps_Vol_3/Update_May_2019/Materials/Mi_EmissiveLight_002.Mi_EmissiveLight_002" :!class /Script/Engine.PrimitiveComponent))
  (Rendering|Material|SetScalarParameterValue _returnvalue "Intensity" (Variables|Default|GetLight_Intensity) :!class /Script/Engine.MaterialInstanceDynamic)
  (Rendering|Lighting|SetAttenuationRadius (Variables|Default|GetPointLight) (Variables|Default|GetAttenuation_Radius)))